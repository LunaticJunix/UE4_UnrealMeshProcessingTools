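; BP_Projectile is a simple projectile actor that flies straight ahead and cleans itself up.
; Each Tick moves it along its forward vector by MoveSpeed scaled by delta time, using SetActorLocation without sweep, so the movement itself does no collision checks.
; It destroys itself once it has existed for more than five seconds; no overlap or hit handling is implemented.
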(event EventBeginPlay)

(event Collision|EventActorBeginOverlap
  (params (OtherActor :type Actor%20Object%20Reference)))

(event EventTick
  (params (DeltaSeconds :type Float%20%28single-precision%29))
  (bind _self self)
  (Transformation|SetActorLocation _self (+ (Transformation|GetActorLocation _self) (* (Transformation|GetActorForwardVector _self) (* DeltaSeconds (Variables|Default|GetMoveSpeed)))) false false)
  (Math|Float|CompareFloat (Actor|GetGameTimeSinceCreation _self) 5.0
    (:>
      (Actor|DestroyActor _self))))

(fn ConstructionScript)