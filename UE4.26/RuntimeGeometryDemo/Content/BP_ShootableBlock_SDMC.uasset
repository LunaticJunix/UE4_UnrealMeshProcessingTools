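; Shootable block that gets carved by projectiles, subtracting each one's mesh from its own when it comes close enough.
; Every Tick it scans all BP_Projectile actors and compares their distance to the block against a quarter of the projectile's bounds extent length.
; Projectiles inside that threshold are passed to SubtractMesh and then destroyed, with no collision events involved.
; An alternative ContainsPoint test is left unconnected and never runs.
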(event EventBeginPlay)

(event Collision|EventActorBeginOverlap
  (params (OtherActor :type Actor%20Object%20Reference)))

(event EventTick
  (params (DeltaSeconds :type Float%20%28single-precision%29))
  (bind _self self)
  (bind _outactors (Actor|GetAllActorsOfClass "/Game/BP_Projectile.BP_Projectile_C"))
  (for _array_element _outactors
    (bind _returnvalue (Class|DynamicMeshBaseActor|DistancetoPoint _self (Transformation|GetActorLocation _array_element)))
    (Math|Float|CompareFloat _returnvalue (* (Math|Vector|VectorLength (.BoxExtent (Collision|GetActorBounds _array_element false false))) 0.25)
      (:<
        (Class|DynamicMeshBaseActor|SubtractMesh _self _array_element)
        (Actor|DestroyActor _array_element)))))

(fn ConstructionScript)